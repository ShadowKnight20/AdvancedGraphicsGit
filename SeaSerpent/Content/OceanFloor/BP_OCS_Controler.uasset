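; BP_OCS_Controler is an OSC receiver in the OceanFloor folder that currently only prints incoming values for debugging.
; On BeginPlay it creates a listening OSC server on a hardcoded local IP and port, then binds a handler to its message-received event.
; The handler prints the first float of each message.
; An unconnected branch for printing the message's address path never runs.
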(event Custom|OSCMessangerReciver
  (params (Message :type OSC%20Message%20Structure%20%28by%20ref%29) (IPAddress :type String) (Port :type Integer))
  (bind _value (Class|OSCManager|GetFloat Message))
  (Development|PrintString (Utilities|String|ToString(Float) _value)))

(event EventBeginPlay
  (bind _returnvalue (Class|OSCManager|CreateOSCServer "192.168.56.1" 1337 false true "" 0))
  (bind _output_get (Variables|Default|SetOSC%20Server _returnvalue))
  (EventDispatchers|BindEventtoOnOscMessageReceived _output_get (EventDispatchers|CreateEvent :!event Custom|OSCMessangerReciver)))

(fn ConstructionScript)